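; BP_Basket is the player-controlled basket that moves sideways and counts the apples it catches.
; On BeginPlay it adds an Enhanced Input mapping context, and IA_Movement moves it along the right vector of the control rotation.
; When an actor stops overlapping TriggerZone, ApplesAmount increases unless that actor is the last one counted.
; IsNotSameActor, despite its name, returns true for a repeat of PreviousActor.
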(event `self.ReceiveBeginPlay`
  (bind _asplayer_controller (cast `PlayerController` (`self.GetController`)))
  (bind _returnvalue (pcsubsystem `EnhancedInputLocalPlayerSubsystem` _asplayer_controller))
  (`/Engine/EditorBlueprintResources/StandardMacros.IsValid` _returnvalue
    (:`Is Valid`
      (message `EnhancedInputSubsystemInterface.AddMappingContext` _returnvalue "/Game/Input/MappingContext.MappingContext" 0 (struct)))))

(event `EnhancedInput|/Game/Input/IA_Movement`
  (params (ActionValue :type "Vector2D Structure") (ElapsedSeconds :type "Float (double-precision)") (TriggeredSeconds :type "Float (double-precision)") (InputAction :type "InputAction Object Reference" :default "/Game/Input/IA_Movement.IA_Movement"))
  (bind (_returnvalue_roll _returnvalue_pitch _returnvalue_yaw) (`KismetMathLibrary.BreakRotator` (`self.GetControlRotation`)))
  (:`Triggered`
    (`self.AddMovementInput` (`KismetMathLibrary.GetRightVector` (`KismetMathLibrary.MakeRotator` _returnvalue_roll 0.0 _returnvalue_yaw)) ActionValue_X)))

(event `self.TriggerZone.OnComponentEndOverlap`
  (params (OverlappedComponent :type "PrimitiveComponent Object Reference") (OtherActor :type "Actor Object Reference") (OtherComp :type "PrimitiveComponent Object Reference") (OtherBodyIndex :type Integer))
  (bind _sameactor (`self.IsNotSameActor` OtherActor))
  (if (not _sameactor)
    (set `self.PreviousActor` OtherActor)
    (set `self.ApplesAmount` (+ (`self.ApplesAmount`) 1))))

(fn `IsNotSameActor`
  (params (Actro1 :type "Actor Object Reference"))
  (returns (SameActor :type Boolean))
  (return (== Actro1 (`self.PreviousActor`))))

(fn `UserConstructionScript`)